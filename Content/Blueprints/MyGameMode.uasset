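; MyGameMode is a game mode that tracks the player's score and decides when the game is won.
; On BeginPlay it creates a MyHUD widget, adds it to the viewport and resets the score to zero.
; UpdateScore adds points to CurrentScore and copies the total into the HUD's Points.
; Tick polls CheckWin every frame, setting HasWon only while the score exactly equals ten.
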(event Custom|Reset
  ;[1 1 1] ResetGame (score)
  (bind _output_get (Variables|/Game/UI/MyHUD.MyHUD_C|SetPoints (Variables|Default|GetHUD) 0))
  (Variables|Default|SetCurrentScore _output_get))

(event Custom|UpdateScore
  (params (Points :type Integer))
  ;[1 1 1] UpdateScore
  (bind _output_get (Variables|Default|SetCurrentScore (+ Points (Variables|Default|GetCurrentScore))))
  (Variables|/Game/UI/MyHUD.MyHUD_C|SetPoints (Variables|Default|GetHUD) _output_get))

(event Custom|CheckWin
  ;[1 1 1] Checks if the score is the winning score and changed bool
  (if (== (Variables|Default|GetCurrentScore) 10)
    (Variables|Default|SethasWon true)
    (else
      (Variables|Default|SethasWon false))))

(event EventBeginPlay
  ;[1 1 1] Add HUD (Score)
  (bind _returnvalue (UserInterface|CreateWidget "/Game/UI/MyHUD.MyHUD_C"))
  (bind _output_get (Variables|Default|SetHUD _returnvalue))
  (UserInterface|Viewport|AddtoViewport _output_get 0)
  (CallFunction|Reset))

(event EventTick
  (params (DeltaSeconds :type Float%20%28single-precision%29))
  (CallFunction|CheckWin))

(fn ConstructionScript)