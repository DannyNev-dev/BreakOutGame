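; BP_Ball is a physics ball that follows the player's arrow until its Launch event fires it with a diagonal impulse.
; Each tick it locks speed to a set value and snaps heading to the nearest horizontal diagonal, keeping it consistent and unstuck.
; It destroys itself when the game mode reports a win.
; On destruction it shows a WinScreen or GameOver widget based on that win state.
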(event Custom|Launch
  ;[1 1 1] Initial Ball Launch Function (Shoots the ball)
  (Variables|Default|SetActive true)
  (Physics|AddImpulse (Variables|Default|GetBall) "700.000000,-700.000000, 0" "None" true))

(event Custom|UpdateBallLocation
  ;[1 1 1] Updates the Balls location when not active
  (if (not (Variables|Default|GetActive))
    (Transformation|SetActorLocation (Transformation|GetWorldLocation (Variables|/Game/Blueprints/BP_Player.BP_Player_C|GetArrow (Variables|Default|GetPlayer))) false false)
    (Transformation|SetActorScale3D "0.500000,0.500000,0.500000")))

(event Custom|VelocityAndAngle
  (bind _returnvalue (Math|Rotator|MakeRotator 0.0 0.0 45.0))
  (bind _speed (Variables|Default|GetSpeed))
  ;[1 1 1] Controls the Angle and speed of the ball (Prevents the ball from getting stuck, Also makes the balls speed consistant and challenging)
  (bind _returnvalue_2 (Physics|GetPhysicsLinearVelocity (Variables|Default|GetBall) "None"))
  (Physics|SetPhysicsLinearVelocity (Variables|Default|GetBall) (* (Math|Vector|UnrotateVector (Math|Rotator|GetRotationXVector (Math|Rotator|MakeRotator 0.0 0.0 (Math|Conversions|ToFloat(Integer) (* (Math|Float|Round (/ (.yaw (Math|Rotator|MakeRotfromX (Math|Vector|RotateVector (Math|Vector|ClampVectorSize _returnvalue_2 _speed _speed) _returnvalue))) 9e+01)) 90)))) _returnvalue) (Math|Vector|VectorLength (Math|Vector|ClampVectorSize _returnvalue_2 _speed _speed))) false "None"))

(event EventBeginPlay
  ;[1 1 1] GetPlayer
  (bind _asbp_player (Utilities|Casting|CastToBP_Player (Pawn|GetControlledPawn (Game|GetPlayerController 0))))
  (Variables|Default|SetPlayer _asbp_player)
  ;[1 1 1] Get game mode
  (bind _asmy_game_mode (Utilities|Casting|CastToMyGameMode (Game|GetGameMode)))
  (Variables|Default|SetGameMode _asmy_game_mode))

(event EventDestroyed
  (if (not (Variables|/Game/Blueprints/MyGameMode.MyGameMode_C|GethasWon (Variables|Default|GetGameMode)))
    (bind _returnvalue (UserInterface|CreateWidget "/Game/UI/GameOver.GameOver_C"))
    (UserInterface|Viewport|AddtoViewport _returnvalue 0)
    (else
      (bind _returnvalue_2 (UserInterface|CreateWidget "/Game/UI/WinScreen.WinScreen_C"))
      (UserInterface|Viewport|AddtoViewport _returnvalue_2 0))))

(event EventTick
  (params (DeltaSeconds :type Float%20%28single-precision%29))
  (CallFunction|UpdateBallLocation)
  ;[1 1 1] Speed and angle function call
  (CallFunction|VelocityandAngle)
  (if (Variables|/Game/Blueprints/MyGameMode.MyGameMode_C|GethasWon (Variables|Default|GetGameMode))
    (Variables|Default|SetActive false)
    (Actor|DestroyActor)))

(fn ConstructionScript)