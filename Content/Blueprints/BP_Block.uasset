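; BP_Block is a breakable, coloured block worth points, destroyed when hit by a BP_Ball.
; Any hit plays a quiet impact sound; a ball hit then waits briefly, destroys the block and passes its truncated Points to MyGameMode's UpdateScore.
; The construction script creates a dynamic material instance from M_Base and sets its Colour parameter from BlockColour.
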(event OnComponentHit(Block)
  (params (HitComponent :type Primitive%20Component%20Object%20Reference) (OtherActor :type Actor%20Object%20Reference) (OtherComp :type Primitive%20Component%20Object%20Reference) (NormalImpulse :type Vector :default "0, 0, 0") (Hit :type Hit%20Result%20Structure%20%28by%20ref%29))
  (Audio|PlaySound2D "/Game/Audio/sfx_sounds_impact11.sfx_sounds_impact11" 0.1 1.0 0.0 0 0)
  (Utilities|Casting|CastToBP_Ball OtherActor)
  (Utilities|FlowControl|Delay 0.1)
  (Actor|DestroyActor)
  (bind _asmy_game_mode (Utilities|Casting|CastToMyGameMode (Game|GetGameMode)))
  (Default|UpdateScore _asmy_game_mode (Math|Float|Truncate (Variables|Default|GetPoints))))

(fn ConstructionScript
  (bind _returnvalue (Rendering|Material|CreateDynamicMaterialInstance (Variables|Default|GetBlock) 0 "/Game/Materials/M_Base.M_Base" "None" :!class /Script/Engine.PrimitiveComponent))
  (Rendering|Material|SetVectorParameterValue _returnvalue "Colour" (Variables|Default|GetBlockColour) :!class /Script/Engine.MaterialInstanceDynamic))