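; BP_Player is the player-controlled paddle that serves and launches balls in what appears to be a Breakout-style game.
; On BeginPlay it runs NewBall, which spawns a BP_Ball at the Arrow component's location and stores it.
; Horizontal axis input pushes the Paddle with physics impulses scaled by Speed, and the Fire action launches the stored ball if it is valid and not yet active.
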(event Custom|NewBall
  (bind _returnvalue (Game|SpawnActorfromClass "/Game/Blueprints/BP_Ball.BP_Ball_C" (Math|Conversions|ToTransform(Vector) (Transformation|GetWorldLocation (Variables|Default|GetArrow))) "Undefined" 0 0))
  (Variables|Default|SetBall _returnvalue))

(event EventBeginPlay
  (CallFunction|NewBall))

(event Input|ActionEvents|InputActionFire
  (params (Key :type Key%20Structure :default "None"))
  (bind _ball (Variables|Default|GetBall))
  (:Pressed
    (if (and (Utilities|IsValid _ball) (not (Variables|/Game/Blueprints/BP_Ball.BP_Ball_C|GetActive _ball)))
      (Default|Launch (Variables|Default|GetBall)))))

(event Input|AxisEvents|InputAxisMoveHorizontal
  (params (AxisValue :type Float%20%28single-precision%29))
  ;[1 1 1] Paddle Movement
  (Physics|AddImpulse (Variables|Default|GetPaddle) (Math|Vector|MakeVector (* AxisValue (Variables|Default|GetSpeed)) 0.0 0.0) "None" false))

(fn ConstructionScript)