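; Physics-driven bouncing ball that launches diagonally on BeginPlay with a velocity-change impulse.
; Every Tick, it forces the velocity magnitude to the Speed variable, keeping pace constant and challenging.
; It also snaps the heading to the nearest horizontal diagonal by rotating 45 degrees, rounding yaw to 90-degree steps and rotating back, which keeps the ball from getting stuck.
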(event Custom|Launch
  ;[1 1 1] Initial Ball Launch Function (Shoots the ball)
  (Physics|AddImpulse (Variables|Default|GetBall) "700.000000,-700.000000, 0" "None" true))

(event Custom|VelocityAndAngle
  (bind _returnvalue (Math|Rotator|MakeRotator 0.0 0.0 45.0))
  (bind _speed (Variables|Default|GetSpeed))
  ;[1 1 1] Controls the Angle and speed of the ball (Prevents the ball from getting stuck, Also makes the balls speed consistant and challenging)
  (bind _returnvalue_2 (Physics|GetPhysicsLinearVelocity (Variables|Default|GetBall) "None"))
  (Physics|SetPhysicsLinearVelocity (Variables|Default|GetBall) (* (Math|Vector|UnrotateVector (Math|Rotator|GetRotationXVector (Math|Rotator|MakeRotator 0.0 0.0 (Math|Conversions|ToFloat(Integer) (* (Math|Float|Round (/ (.yaw (Math|Rotator|MakeRotfromX (Math|Vector|RotateVector (Math|Vector|ClampVectorSize _returnvalue_2 _speed _speed) _returnvalue))) 9e+01)) 90)))) _returnvalue) (Math|Vector|VectorLength (Math|Vector|ClampVectorSize _returnvalue_2 _speed _speed))) false "None"))

(event EventBeginPlay
  ;[1 1 1] Launch Ball function call
  (CallFunction|Launch))

(event EventTick
  (params (DeltaSeconds :type Float%20%28single-precision%29))
  ;[1 1 1] Speed and angle function call
  (CallFunction|VelocityandAngle))

(fn ConstructionScript)